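; BP_Socket is a test actor that receives JSON data over UDP and prints it for debugging.
; On BeginPlay it opens a receive socket on localhost port 12345 and prints the result.
; Each received packet is converted to a string, deserialized into a Params struct, and its integer, bool, string and float arrays are printed in turn, each followed by a type label.
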(event OnReceivedBytes(UDP)
  (params (Bytes :type Array%20of%20Bytes) (IPAddress :type String) (Port :type Integer%20%28by%20ref%29))
  (bind _returnvalue (Class|JsonDeserializer|JsonDeserialize (Class|CUBlueprintLibrary|ToString(Bytes) Bytes)))
  (bind _output_get (Variables|Default|SetParams _returnvalue))
  (Utilities|FlowControl|Sequence
    (:then_0
      (for _array_element (.intToReceive (Utilities|Struct|BreakParameters _output_get))
        (Development|PrintString (Utilities|String|ToString(Integer) _array_element) true true "(R=0.000000,G=0.660000,B=1.000000,A=1.000000)" 1e+03))
      (Development|PrintString "Integers" true true "(R=0.000000,G=1.000000,B=0.888978,A=1.000000)" 1e+03))
    (:then_1
      (for _array_element_2 (.boolToReceive (Utilities|Struct|BreakParameters _output_get))
        (Development|PrintString (Utilities|String|ToString(Boolean) _array_element_2) true true "(R=0.000000,G=0.660000,B=1.000000,A=1.000000)" 1e+03))
      (Development|PrintString "Bools" true true "(R=1.000000,G=0.000000,B=0.027538,A=1.000000)" 1e+03))
    (:then_2
      (for _array_element_3 (.stringToReceive (Utilities|Struct|BreakParameters _output_get))
        (Development|PrintString _array_element_3 true true "(R=0.000000,G=0.660000,B=1.000000,A=1.000000)" 1e+03))
      (Development|PrintString "Strings" true true "(R=0.913570,G=0.000000,B=1.000000,A=1.000000)" 1e+03))
    (:then_3
      (for _array_element_4 (.floatToReceive (Utilities|Struct|BreakParameters _output_get))
        (Development|PrintString (Utilities|String|ToString(Float) _array_element_4) true true "(R=0.000000,G=0.660000,B=1.000000,A=1.000000)" 1e+03))
      (Development|PrintString "Floats" true true "(R=0.080374,G=1.000000,B=0.000000,A=1.000000)" 1e+03))))

(event EventBeginPlay
  (bind _returnvalue (Class|UDPComponent|OpenReceiveSocket (Variables|Default|GetUDP) "127.0.0.1" 12345))
  (Development|PrintString (Utilities|String|ToString(Boolean) _returnvalue)))

(event Collision|EventActorBeginOverlap
  (params (OtherActor :type Actor%20Object%20Reference)))

(event EventTick
  (params (DeltaSeconds :type Float%20%28single-precision%29)))

(fn ConstructionScript)